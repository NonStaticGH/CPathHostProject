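; Debug test actor for threading that reports sent and received request counts on screen.
; On BeginPlay, only the instance with one hardcoded display name enables printing and starts a looping one-second timer, so a single actor reports.
; The timer event prints the two request counters, which this graph reads but never updates.
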(event `self.ReceiveBeginPlay`
  (bind _output_get (set `self.ShouldPrint` (`KismetStringLibrary.EqualEqual_StrStr` (`KismetSystemLibrary.GetDisplayName` self) "BP_NewThreadingTest214")))
  (if _output_get
    (`KismetSystemLibrary.K2_SetTimerDelegate` (delegate `CustomEvent_0`) 1.0 true)))

(event `CustomEvent_0`
  (if (`self.ShouldPrint`)
    (`KismetSystemLibrary.PrintString` (`KismetStringLibrary.Concat_StrStr` "Sent: " (`KismetStringLibrary.Conv_IntToString` (`self.RequestsSentBP`))) true true (struct :`G` 0.66 :`B` 1.0 :`A` 1.0) 1.0)
    (`KismetSystemLibrary.PrintString` (`KismetStringLibrary.Concat_StrStr` "Received: " (`KismetStringLibrary.Conv_IntToString` (`self.RequestsReceivedBP`))) true true (struct :`G` 0.66 :`B` 1.0 :`A` 1.0) 1.0)))

(event `self.ReceiveTick`
  (params (DeltaSeconds :type "Float (single-precision)")))

(fn `UserConstructionScript`)